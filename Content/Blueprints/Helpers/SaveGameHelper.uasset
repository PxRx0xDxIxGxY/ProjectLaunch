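; Helper Blueprint that saves and loads player game settings (master, music and SFX volume plus a graphics quality level) through a GameSettings SaveGame object.
; SaveGameSettings writes the values into a new object and saves it to the slot name and index defined on that class.
; LoadGameSettings creates a temporary object to read that slot, then returns the saved values, or saves and returns hardcoded defaults when no save exists.
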(fn `LoadGameSettings`
  (returns (MasterVolume :type "Float (double-precision)") (MusicVolume :type "Float (double-precision)") (SFXVolume :type "Float (double-precision)") (GraphicsSettings :type Integer))
  (bind _savegamesettingsreference (`self.SaveGameSettingsReference`))
  (bind _saveslotname (`/Game/Blueprints/GameSaveObjects/GameSettings.SaveSlotName` _savegamesettingsreference))
  (bind _saveindex (`/Game/Blueprints/GameSaveObjects/GameSettings.SaveIndex` _savegamesettingsreference))
  (bind _returnvalue (`GameplayStatics.CreateSaveGameObject` "/Game/Blueprints/GameSaveObjects/GameSettings.GameSettings_C"))
  (bind _asgame_settings (cast `/Game/Blueprints/GameSaveObjects/GameSettings` _returnvalue))
  (set `self.SaveGameSettingsReference` _asgame_settings)
  (bind _returnvalue_2 (`GameplayStatics.DoesSaveGameExist` _saveslotname _saveindex))
  (if _returnvalue_2
    (bind _returnvalue_3 (`GameplayStatics.LoadGameFromSlot` _saveslotname _saveindex))
    (bind _asgame_settings_2 (cast `/Game/Blueprints/GameSaveObjects/GameSettings` _returnvalue_3))
    (set `self.SaveGameSettingsReference` _asgame_settings_2)
    (return (`/Game/Blueprints/GameSaveObjects/GameSettings.MasterVolume` _asgame_settings_2) (`/Game/Blueprints/GameSaveObjects/GameSettings.MusicVolume` _asgame_settings_2) (`/Game/Blueprints/GameSaveObjects/GameSettings.SFXVolume` _asgame_settings_2) (`/Game/Blueprints/GameSaveObjects/GameSettings.GraphicsSettings` _asgame_settings_2))
    (else
      (`self.SaveGameSettings` 1.0 1.0 1.0 3)
      (return 1.0 1.0 1.0 3))))

(fn `SaveGameSettings`
  (params (MasterVolume :type "Float (double-precision)") (MusicVolume :type "Float (double-precision)") (SFXVolume :type "Float (double-precision)") (`GraphicsSettings (0-3)` :type Integer))
  (bind _savegamesettingsreference (`self.SaveGameSettingsReference`))
  (bind _returnvalue (`GameplayStatics.CreateSaveGameObject` "/Game/Blueprints/GameSaveObjects/GameSettings.GameSettings_C"))
  (bind _asgame_settings (cast `/Game/Blueprints/GameSaveObjects/GameSettings` _returnvalue))
  (set `self.SaveGameSettingsReference` _asgame_settings)
  (set `/Game/Blueprints/GameSaveObjects/GameSettings.MasterVolume` MasterVolume _savegamesettingsreference)
  (set `/Game/Blueprints/GameSaveObjects/GameSettings.MusicVolume` MusicVolume _savegamesettingsreference)
  (set `/Game/Blueprints/GameSaveObjects/GameSettings.SFXVolume` SFXVolume _savegamesettingsreference)
  (set `/Game/Blueprints/GameSaveObjects/GameSettings.GraphicsSettings` `GraphicsSettings (0-3)` _savegamesettingsreference)
  (`GameplayStatics.SaveGameToSlot` _savegamesettingsreference (`/Game/Blueprints/GameSaveObjects/GameSettings.SaveSlotName` _savegamesettingsreference) (`/Game/Blueprints/GameSaveObjects/GameSettings.SaveIndex` _savegamesettingsreference)))