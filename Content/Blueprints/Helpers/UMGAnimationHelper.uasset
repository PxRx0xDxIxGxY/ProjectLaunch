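; UMG animation helper with a single function, ShowMenuAnimation, that shows or hides a menu by driving a widget animation forward or backward.
; It compares the requested activation with the caller's Direction flag, does nothing when they match, and returns the resulting direction.
; Showing plays forward from the animation's current time.
; Hiding reverses an animation in progress, or otherwise plays it in reverse from the current time.
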(fn `ShowMenuAnimation`
  (params (WidgetReference :type "UserWidget Object Reference") (Animation :type "WidgetAnimation Object Reference") (AnimationSpeed :type "Float (double-precision)") (ActivateAnimation :type Boolean) (Direction :type Boolean))
  (returns (NewDirection :type Boolean))
  (bind _returnvalue (not Direction))
  (bind _returnvalue_2 (`UserWidget.GetAnimationCurrentTime` WidgetReference Animation))
  (if ActivateAnimation
    (if _returnvalue
      (`UserWidget.PlayAnimation` WidgetReference Animation _returnvalue_2 1 "Forward" AnimationSpeed)
      (return true)
      (else
        _))
    (elif Direction
      (if (`UserWidget.IsAnimationPlaying` WidgetReference Animation)
        (`UserWidget.ReverseAnimation` WidgetReference Animation)
        (return _returnvalue)
        (else
          (`UserWidget.PlayAnimation` WidgetReference Animation _returnvalue_2 1 "Reverse" AnimationSpeed)
          (return false)))
      (else
        _)))
  (return Direction))