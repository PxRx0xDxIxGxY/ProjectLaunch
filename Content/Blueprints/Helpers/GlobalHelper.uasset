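; GlobalHelper is an actor Blueprint that acts as a thin facade over the mouse, UMG animation and audio helpers.
; It forwards the mouse-on-left query to MouseHelper and menu animation requests to UMGAnimationHelper, supplying its own MenuAnimationSpeed.
; Its volume functions write master, music and SFX values directly into AudioHelper variables, with music stored as MusicAudio.
; The event graph and construction script contain no logic.
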(event `self.ReceiveTick`
  (params (DeltaSeconds :type "Float (single-precision)")))

(fn `IsMouseOnLeft`
  (returns (IsMouseOnLeft :type Boolean))
  (bind _ismouseonleft (`/Game/Blueprints/Helpers/MouseHelper.IsMouseOnLeft` (`self.MouseHelper`)))
  (return _ismouseonleft))

(fn `ShowMenuAnimation`
  (params (Widget :type "UserWidget Object Reference") (WidgetAnimation :type "WidgetAnimation Object Reference") (ActivateAnimation :type Boolean) (Direction :type Boolean))
  (returns (NewDirection :type Boolean))
  (bind _newdirection (`/Game/Blueprints/Helpers/UMGAnimationHelper.ShowMenuAnimation` (`self.UMGAnimationHelper`) Widget WidgetAnimation (`self.MenuAnimationSpeed`) ActivateAnimation Direction))
  (return _newdirection))

(fn `UpdateMasterVolume`
  (params (`New Volume` :type "Float (double-precision)"))
  (set `/Game/Blueprints/Helpers/AudioHelper.MasterVolume` `New Volume` (`self.AudioHelper`)))

(fn `UpdateMusicVolume`
  (params (`New Volume` :type "Float (double-precision)"))
  (set `/Game/Blueprints/Helpers/AudioHelper.MusicAudio` `New Volume` (`self.AudioHelper`)))

(fn `UpdateSFXVolume`
  (params (NewVolume :type "Float (double-precision)"))
  (set `/Game/Blueprints/Helpers/AudioHelper.SFXVolume` NewVolume (`self.AudioHelper`)))

(fn `UserConstructionScript`)