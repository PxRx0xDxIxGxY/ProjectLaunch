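; Player controller for the main menu that sets up the menu UI when play begins.
; On BeginPlay it spawns a GlobalHelper actor at the world origin and stores it.
; It then creates the MainMenu widget, hands it the GlobalHelper reference and adds it to the viewport.
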(event `self.ReceiveBeginPlay`
  (`self.CreateGlobalHelper`)
  (`self.InitializeMainMenuWidget`))

(event `self.ReceiveTick`
  (params (DeltaSeconds :type "Float (single-precision)")))

(fn `CreateGlobalHelper`
  (bind _returnvalue (`|SpawnActorFromClass` "/Game/Blueprints/Helpers/GlobalHelper.GlobalHelper_C" (`KismetMathLibrary.MakeTransform` (0.0 0.0 0.0)) "Undefined" "OverrideRootScale"))
  (set `self.GlobalHelper` _returnvalue))

(fn `InitializeMainMenuWidget`
  (bind _returnvalue (`|CreateWidget` "/Game/UMG/MainMenu.MainMenu_C"))
  (bind _output_get (set `self.MainMenuWidget` _returnvalue))
  (set `/Game/UMG/MainMenu.GlobalHelper` (`self.GlobalHelper`) _output_get)
  (`UserWidget.AddToViewport` _output_get 0))

(fn `UserConstructionScript`)